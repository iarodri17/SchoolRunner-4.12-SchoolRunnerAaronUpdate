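; Pickup actor that spins in place and is collected when the player touches it.
; The construction script applies a configurable static mesh, and Tick yaws the actor at RotationRate scaled by delta time.
; When the sphere collider overlaps player character 0, it sends CollectedPickupsMessage with a fixed enum value to the game mode, then destroys itself.
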(event OnComponentBeginOverlap(SphereCollider)
  (params (OverlappedComponent :type Primitive%20Component%20Object%20Reference) (OtherActor :type Actor%20Object%20Reference) (OtherComp :type Primitive%20Component%20Object%20Reference) (OtherBodyIndex :type Integer) (bFromSweep :type Boolean) (SweepResult :type Hit%20Result%20Structure%20%28by%20ref%29))
  ;[1 1 1] Player Collision
  (if (== (Game|GetPlayerCharacter 0) OtherActor)
    (Class|BPIGameMode|CollectedPickups(Message) (Game|GetGameMode) "NewEnumerator1")
    (Actor|DestroyActor)))

(event EventTick
  (params (DeltaSeconds :type Float%20%28single-precision%29))
  ;[1 1 1] Rotation Rate
  (Transformation|AddActorLocalRotation (Math|Rotator|MakeRotator 0.0 0.0 (* (Variables|Default|GetRotationRate) DeltaSeconds)) false false))

(fn ConstructionScript
  (Components|StaticMesh|SetStaticMesh (Variables|Default|GetPickupMesh) (Variables|Default|GetStaticMeshToDisplay)))